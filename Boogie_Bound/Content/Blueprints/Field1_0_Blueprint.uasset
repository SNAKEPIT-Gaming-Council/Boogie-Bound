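; Field1_0 is a field Blueprint that temporarily places an Obstacle_Ring at one of three random points.
; BeginPlay runs two spawn-then-destroy cycles on fixed delays, with no further looping.
; SpawnObstacles stores the new ring and sets a flag for the chosen point.
; DestroyObstacles removes the ring of the first flagged point in order, and nothing clears the flags between cycles.
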(event EventBeginPlay
  (Utilities|FlowControl|Delay 3.0)
  (CallFunction|SpawnObstacles)
  (Utilities|FlowControl|Delay 3.0)
  (CallFunction|DestroyObstacles)
  (Utilities|FlowControl|Delay 3.0)
  (CallFunction|SpawnObstacles)
  (Utilities|FlowControl|Delay 3.0)
  (CallFunction|DestroyObstacles))

(event Collision|EventActorBeginOverlap
  (params (OtherActor :type Actor%20Object%20Reference)))

(event EventTick
  (params (DeltaSeconds :type Float%20%28single-precision%29)))

(fn ConstructionScript)

(fn SpawnObstacles
  (switch int (Math|Random|RandomIntegerinRange 0 2)
    (:0
      (bind _returnvalue (Game|SpawnActorfromClass "/Game/Blueprints/Obstacle_Ring.Obstacle_Ring_C" (Transformation|GetWorldTransform (Variables|Default|GetPoint1)) "Undefined" 0 0))
      (Variables|Default|Setpoint_1 _returnvalue)
      (Variables|Default|Setpoint__1 true))
    (:1
      (bind _returnvalue_2 (Game|SpawnActorfromClass "/Game/Blueprints/Obstacle_Ring.Obstacle_Ring_C" (Transformation|GetWorldTransform (Variables|Default|GetPoint2)) "Undefined" 0 0))
      (Variables|Default|Setpoint_2 _returnvalue_2)
      (Variables|Default|Setpoint__2 true))
    (:2
      (bind _returnvalue_3 (Game|SpawnActorfromClass "/Game/Blueprints/Obstacle_Ring.Obstacle_Ring_C" (Transformation|GetWorldTransform (Variables|Default|GetPoint3)) "Undefined" 0 0))
      (Variables|Default|Setpoint_3 _returnvalue_3)
      (Variables|Default|Setpoint__3 true))))

(fn DestroyObstacles
  (if (Variables|Default|Getpoint__1)
    (Actor|DestroyActor (Variables|Default|Getpoint_1))
    (elif (Variables|Default|Getpoint__2)
      (Actor|DestroyActor (Variables|Default|Getpoint_2))
      (elif (Variables|Default|Getpoint__3)
        (Actor|DestroyActor (Variables|Default|Getpoint_3))))))